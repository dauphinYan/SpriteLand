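; PC_SpriteLand is a player controller Blueprint that manages the backpack UI.
; On BeginPlay it creates a W_Backpack widget and stores it in NewVar without displaying it.
; The DebugKeyF press toggles that same widget in and out of the viewport, showing the mouse cursor only while the backpack is open.
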(event EventBeginPlay
  (bind _returnvalue (UserInterface|CreateWidget "/Game/Blueprint/UMG/Backpack/W_Backpack.W_Backpack_C"))
  (Variables|Default|SetNewVar _returnvalue))

(event EventTick
  (params (DeltaSeconds :type Float%20%28single-precision%29)))

(event Input|KeyboardEvents|DebugKeyF
  (params (Key :type Key%20Structure :default "None") (ActionValue :type Input%20Action%20Value%20Structure))
  (:Pressed
    (if (UserInterface|Viewport|IsinViewport (Variables|Default|GetNewVar))
      (Widget|RemovefromParent (Variables|Default|GetNewVar))
      (Variables|Default|SetbShowMouseCursor false)
      (else
        (UserInterface|Viewport|AddtoViewport (Variables|Default|GetNewVar) 0)
        (Variables|Default|SetbShowMouseCursor true)))))

(fn ConstructionScript)